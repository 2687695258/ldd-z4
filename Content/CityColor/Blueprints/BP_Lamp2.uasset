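; BP_Lamp2 is an interactive lamp that shows a widget and accepts control events only while an actor overlaps it.
; Open and ChangeColor use FlipFlops to toggle the mesh material's emissive strength between off and on, and its color between warm amber and white.
; EnhanceBrightness and ReduceBrightness step a clamped brightness value, with Timelines lerping the emissive parameter to the new target.
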(event EventBeginPlay
  (Rendering|SetVisibility (Variables|Default|GetWidget) false false))

(event Collision|EventActorBeginOverlap
  (params (OtherActor :type Actor%20Object%20Reference))
  (Variables|Default|SetOverlap true)
  (Rendering|SetVisibility (Variables|Default|GetWidget) true false))

(event EventOpen
  (bind _staticmesh (Variables|Default|GetStaticMesh))
  (if (Variables|Default|GetOverlap)
    (Utilities|FlowControl|FlipFlop
      (:A
        (Rendering|Material|SetScalarParameterValueonMaterials _staticmesh "Light Emissive Strength" 0.0))
      (:B
        (Rendering|Material|SetScalarParameterValueonMaterials _staticmesh "Light Emissive Strength" 2.0)))))

(event EventEnhanceBrightness
  (if (Variables|Default|GetOverlap)
    (Variables|Default|SetTarget%20Light%20Brightness (Math|Float|Clamp(Float) (+ (Variables|Default|GetCurrrent%20Light%20Brightness) 2.0) 1.0 12.0))
    (bind _新建轨道_0 (Timeline|时间轴_0 Play)
      (:Update
        (Rendering|Material|SetScalarParameterValueonMaterials (Variables|Default|GetStaticMesh) "Light Emissive Strength" (Math|Float|Lerp (Variables|Default|GetCurrrent%20Light%20Brightness) (Variables|Default|GetTarget%20Light%20Brightness) _新建轨道_0)))
      (:Finished
        (Variables|Default|SetCurrrent%20Light%20Brightness (Variables|Default|GetTarget%20Light%20Brightness))))))

(event Collision|EventActorEndOverlap
  (params (OtherActor :type Actor%20Object%20Reference))
  (Variables|Default|SetOverlap false)
  (Rendering|SetVisibility (Variables|Default|GetWidget) false false))

(event EventChangeColor
  (bind _staticmesh (Variables|Default|GetStaticMesh))
  (if (Variables|Default|GetOverlap)
    (Utilities|FlowControl|FlipFlop
      (:A
        (Rendering|Material|SetVectorParameterValueonMaterials _staticmesh "LightEmissiveColor" "0.650000,0.360000,0.030000"))
      (:B
        (Rendering|Material|SetVectorParameterValueonMaterials _staticmesh "LightEmissiveColor" "1.000000,1.000000,1.000000")))))

(event EventReduceBrightness
  (if (Variables|Default|GetOverlap)
    (Variables|Default|SetTarget%20Light%20Brightness (Math|Float|Clamp(Float) (- (Variables|Default|GetCurrrent%20Light%20Brightness) 2.0) 1.0 12.0))
    (bind _新建轨道_0 (Timeline|时间轴_1 Play)
      (:Update
        (Rendering|Material|SetScalarParameterValueonMaterials (Variables|Default|GetStaticMesh) "Light Emissive Strength" (Math|Float|Lerp (Variables|Default|GetCurrrent%20Light%20Brightness) (Variables|Default|GetTarget%20Light%20Brightness) _新建轨道_0)))
      (:Finished
        (Variables|Default|SetCurrrent%20Light%20Brightness (Variables|Default|GetTarget%20Light%20Brightness))))))

(fn ConstructionScript)